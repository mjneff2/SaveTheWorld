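; BP_MapGrid is a map actor that spawns a square grid of BP_GridSquare blocks when play begins.
; A single loop over Size squared indices uses modulo and division by Size to turn each index into X and Y coordinates.
; Each coordinate is scaled by BlockSpacing and offset from the grid actor's location, so the layout extends from that point on a flat plane.
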(event EventBeginPlay
  (bind _blockspacing (Variables|Default|GetBlockSpacing))
  (bind _size (Variables|Default|GetSize))
  (bind _size_2 (Variables|Default|GetSize))
  (for _index (range 0 (- (* _size _size) 1)) ; Loop to spawn each block
    (Game|SpawnActorfromClass "/Game/Blueprints/Map/BP_GridSquare.BP_GridSquare_C" (Math|Conversions|ToTransform(Vector) (+ (Math|Vector|MakeVector (* (Math|Integer|%(Integer) _index _size_2) _blockspacing) (* (/ _index _size_2) _blockspacing) 0.0) (Transformation|GetActorLocation))) "Undefined" 0 0)))

(fn ConstructionScript)