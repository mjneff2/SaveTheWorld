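; BP_GridSquare is a map tile for placing towers, such as in a tower defense grid.
; Clicking its Cube component spawns a BP_TowerBase just above it, provided the square is Buildable and has no tower yet.
; It then sets HasTower to block repeat placement and prints the clicked component's name.
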(event OnClicked(Cube)
  (params (TouchedComponent :type Primitive%20Component%20Object%20Reference) (ButtonPressed :type Key%20Structure :default "None"))
  (bind _returnvalue (Transformation|GetWorldLocation TouchedComponent))
  (if (and (Variables|Default|GetBuildable) (not (Variables|Default|GetHasTower)))
    (Game|SpawnActorfromClass "/Game/Blueprints/Towers/BP_TowerBase.BP_TowerBase_C" (Math|Transform|MakeTransform (Math|Vector|MakeVector (.x _returnvalue) (.y _returnvalue) (+ (.z _returnvalue) 1e+02)) "0, 0, 0" "1,1,1") "Undefined" 0 0)
    (Variables|Default|SetHasTower true)
    (Development|PrintString (Utilities|GetDisplayName TouchedComponent))))

(event EventBeginPlay)

(event Collision|EventActorBeginOverlap
  (params (OtherActor :type Actor%20Object%20Reference)))

(event EventTick
  (params (DeltaSeconds :type Float%20%28single-precision%29)))

(fn ConstructionScript)